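; BP_Data is a data Blueprint that builds TexDic, a lookup of image textures keyed by asset name.
; ReloadData clears the map, then queries the Asset Registry recursively under /Game/Assets/Images, including in-memory assets.
; It resolves each result with GetAsset and adds only those that cast to Texture2D.
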(event `Reload Data`
  (`BlueprintMapLibrary.Map_Clear` (`self.TexDic`))
  (bind _outassetdata (`AssetRegistry.GetAssetsByPath` (`AssetRegistryHelpers.GetAssetRegistry`) "/Game/Assets/Images" true false))
  (for _array_element _outassetdata
    (bind _astexture_2d (cast `Texture2D` (`AssetRegistryHelpers.GetAsset` _array_element)))
    (`BlueprintMapLibrary.Map_Add` (`self.TexDic`) (`KismetStringLibrary.Conv_NameToString` (`.AssetName` (break `AssetData` _array_element))) _astexture_2d)))